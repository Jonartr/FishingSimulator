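; BP_Pescar is a spawner that fills a box volume with Pescadito actors (little fish, by name) when play begins.
; BeginPlay spawns Num instances at random points inside the Box component's scaled extent, each with a random yaw, and stores them in the Flock array.
; It contains no movement or flocking logic, as Tick and overlap events are disabled and the construction script is empty.
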(event `self.ReceiveBeginPlay`
  (for _ (range (`self.Num`))
    (bind _returnvalue (`|SpawnActorFromClass` "/Game/Fish/Pescadito.Pescadito_C" (`KismetMathLibrary.MakeTransform` (`KismetMathLibrary.RandomPointInBoundingBox` (`SceneComponent.K2_GetComponentLocation` (`self.Box`)) (`BoxComponent.GetScaledBoxExtent` (`self.Box`))) (`KismetMathLibrary.MakeRotator` 0.0 0.0 (`KismetMathLibrary.RandomFloatInRange` 0.0 360.0))) "Undefined" "MultiplyWithRoot" null null))
    (`KismetArrayLibrary.Array_Add` (`self.Flock`) _returnvalue)))

(fn `UserConstructionScript`)